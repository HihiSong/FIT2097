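; BP_Remote is a switch actor that remotely operates a BP_RomoteDoor.
; Its OpenDoor event swaps visibility between the Upperswitch and Lowerswitch components, then calls OpenDoor on the door indexed by NoRemote in a GetAllActorsOfClass result.
; Matching turnoff and remoteOff events restore the switch and close that door, but nothing in this graph calls them.
; Door pairing depends on the order of that actor array rather than a direct reference.
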(event Custom|turnon
  ;[1 1 1] on
  (Rendering|SetVisibility (Variables|Default|Getupperswitch) false false)
  (Rendering|SetVisibility (Variables|Default|Getlowerswitch) true false))

(event Custom|OpenDoor
  (CallFunction|Turnon)
  (CallFunction|Remoteon))

(event Custom|turnoff
  ;[1 1 1] off
  (Rendering|SetVisibility (Variables|Default|Getupperswitch) true false)
  (Rendering|SetVisibility (Variables|Default|Getlowerswitch) false false))

(event Custom|remoteOff
  (bind _outactors (Actor|GetAllActorsOfClass "/Game/Assets/Actor/BP_RomoteDoor.BP_RomoteDoor_C"))
  (Default|CloseDoor (Utilities|Array|Get(acopy) _outactors (Variables|Default|GetNoRemote))))

(event Custom|remoteOn
  (bind _outactors (Actor|GetAllActorsOfClass "/Game/Assets/Actor/BP_RomoteDoor.BP_RomoteDoor_C"))
  (Default|OpenDoor (Utilities|Array|Get(acopy) _outactors (Variables|Default|GetNoRemote))))

(event EventBeginPlay)

(event Collision|EventActorBeginOverlap
  (params (OtherActor :type Actor%20Object%20Reference)))

(event EventTick
  (params (DeltaSeconds :type Float%20%28single-precision%29)))

(fn ConstructionScript)