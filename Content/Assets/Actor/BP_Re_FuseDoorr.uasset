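; BP_Re_FuseDoorr is an actor Blueprint whose only logic here visualizes its network relevancy radius.
; On BeginPlay it calls the parent, then scales RelerancyRadiusMesh in X and Y by the square root of NetCullDistanceSquared divided by 50, keeping Z at 1.
; Overlap and Tick are disabled stubs, the construction script only calls its parent, and no door or fuse behavior appears in these graphs.
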(event EventBeginPlay
  (bind _netculldistancesquared (Variables|Default|GetNetCullDistanceSquared))
  (bind _returnvalue (Math|Float|Sqrt _netculldistancesquared))
  (bind _returnvalue_2 (/ _returnvalue 5e+01))
  (|CallParentFunction)
  (Transformation|SetWorldScale3D (Variables|Default|GetRelerancyRadiusMesh) (Math|Vector|MakeVector _returnvalue_2 _returnvalue_2 1.0)))

(event Collision|EventActorBeginOverlap
  (params (OtherActor :type Actor%20Object%20Reference))
  (|CallParentFunction OtherActor) ; This node is disabled and will not be called.\nDrag off pins to build functionality.
)

(event EventTick
  (params (DeltaSeconds :type Float%20%28single-precision%29))
  (|CallParentFunction DeltaSeconds) ; This node is disabled and will not be called.\nDrag off pins to build functionality.
)

(fn ConstructionScript
  (|CallParentFunction))