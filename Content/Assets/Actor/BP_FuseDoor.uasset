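; BP_FuseDoor is a locked door actor that opens when its OpenDoor event is called.
; It starts locked, then a timeline rotates an arrow component to swing the door and clears the Locked flag.
; Opening also reveals the fuse mesh on its box and, via a DoOnce, spawns an attached particle effect and plays a collapse sound.
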(event EventBeginPlay
  (|CallParentFunction)
  (Variables|Default|SetLocked true))

(event Collision|EventActorBeginOverlap
  (params (OtherActor :type Actor%20Object%20Reference))
  (|CallParentFunction OtherActor) ; This node is disabled and will not be called.\nDrag off pins to build functionality.
)

(event EventTick
  (params (DeltaSeconds :type Float%20%28single-precision%29))
  (|CallParentFunction DeltaSeconds) ; This node is disabled and will not be called.\nDrag off pins to build functionality.
)

(event EventOpenDoor
  ;[1 1 1] open door
  (bind _open (Timeline|Timeline_1 Play)
    (:Update
      (Transformation|SetRelativeRotation (Variables|Default|GetArrow) (Math|Rotator|Lerp(Rotator) "0, 0, 0" "0,90.000000, 0" _open) false false)
      (Variables|Default|SetLocked false)
      ;[1 1 1] display fuse on box
      (Rendering|SetVisibility (Variables|Default|GetStaticMesh) true false)
      ;[1 1 1] spawn particle
      (Utilities|FlowControl|DoOnce false
        (:Completed
          (Effects|SpawnEmitterAttached "/Game/Assets/Particle/OpenFuseDoor.OpenFuseDoor" (Variables|Default|GetStaticMesh1) "None")
          ;[1 1 1] play sound
          (Audio|PlaySound2D "/Game/StarterContent/Audio/Collapse01.Collapse01"))))))

(fn ConstructionScript
  (|CallParentFunction))