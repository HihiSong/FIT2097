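; BP_NormalDoor is a door actor that can be opened and shows whether it is locked.
; OpenDoor plays a timeline that lerps the Arrow component's relative rotation toward a 90 degree turn, clearing the Locked flag during the update.
; Tick refreshes a text render every frame with the locked or unlocked message.
; BeginPlay sets the Name variable from OwnName.
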(event Custom|OpenDoor
  ;[1 1 1] open door function
  (bind _open (Timeline|Timeline_0 Play)
    (:Update
      (Transformation|SetRelativeRotation (Variables|Default|GetArrow) (Math|Rotator|Lerp(Rotator) "0, 0, 0" "0,90.000000, 0" _open) false false)
      (Variables|Default|SetLocked false))))

(event Custom|textCheckLock
  (bind _textrender (Variables|Default|GetTextRender))
  ;[1 1 1] message show door is lock or not
  (if (Variables|Default|GetLocked)
    (Rendering|Components|TextRender|SetText _textrender (Variables|Default|GetmessageLock))
    (else
      (Rendering|Components|TextRender|SetText _textrender (Variables|Default|GetmessageUnlock)))))

(event EventBeginPlay
  ;[1 1 1] set name
  (Variables|Default|SetName (Variables|Default|GetOwnName)))

(event Collision|EventActorBeginOverlap
  (params (OtherActor :type Actor%20Object%20Reference)))

(event EventTick
  (params (DeltaSeconds :type Float%20%28single-precision%29))
  (CallFunction|TextCheckLock))

(fn ConstructionScript)